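; BP_SecurityCam is a security camera that raises an alarm for enemy AI when it senses a target.
; HandleSight takes a sight result and, on detection, turns the mesh red, plays a sound at the camera and prints a debug message.
; It then passes the stimulus location to every BP_StupidEnemy in the level through CheckSecurityAlarm.
; Losing the target only turns the mesh green and prints a message.
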(fn `HandleSight`
  (params (Target :type "Actor Object Reference") (`Successfully Sensed` :type Boolean) (`Stimulus Location` :type "Vector Structure"))
  (if `Successfully Sensed`
    (`KismetSystemLibrary.PrintText` "Aquired Target")
    (`PrimitiveComponent.SetMaterial` (`self.StaticMesh`) 0 "/AnimationSharing/AnimSharingRed.AnimSharingRed")
    (`GameplayStatics.PlaySoundAtLocation` "/Engine/EditorSounds/Notifications/CompileFailed.CompileFailed" (`self.K2_GetActorLocation`) (struct) 1.0 1.0 0.0 "/Game/SFX/ATT_Default.ATT_Default" null null null)
    (bind _outactors (`GameplayStatics.GetAllActorsOfClass` "/Game/Blueprints/EnemyAI/BP_StupidEnemy.BP_StupidEnemy_C"))
    (for _array_element _outactors
      (`/Game/Blueprints/EnemyAI/BP_StupidEnemy.Check Security Alarm` _array_element `Stimulus Location`))
    (else
      (`KismetSystemLibrary.PrintText` "Lost Target")
      (`PrimitiveComponent.SetMaterial` (`self.StaticMesh`) 0 "/AnimationSharing/AnimSharingGreen.AnimSharingGreen"))))

(fn `UserConstructionScript`)