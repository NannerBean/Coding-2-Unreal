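; BP_Turret is an enemy turret that rotates every tick to face its target and fires BP_Bullet projectiles.
; HandleSight stores the sensed target and starts a Tracking-Attacking loop that fires every second.
; Losing sight only clears TrackingTarget, which neither rotation nor the loop checks.
; Bullets spawn at BulletSpawn's relative transform, and their impulse node is disconnected.
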(event `Fire Projectile`
  (bind _returnvalue (`|SpawnActorFromClass` "/Game/Blueprints/EnemyAI/BP_Bullet.BP_Bullet_C" (`SceneComponent.GetRelativeTransform` (`self.Bullet Spawn`)) "Undefined" "MultiplyWithRoot" null null)))

(event `self.ReceiveTick`
  (params (DeltaSeconds :type "Float (single-precision)"))
  (`self.K2_SetActorRotation` (`KismetMathLibrary.FindLookAtRotation` (`self.K2_GetActorLocation`) (`self.K2_GetActorLocation` (`self.Target`)))))

(event `Handle Sight`
  (params (Target :type "Actor Object Reference") (Sensed :type Boolean))
  (if Sensed
    (set `self.Target` Target)
    (`self.Tracking`)
    (else
      (`self.Looking`))))

(event `Looking`
  (set `self.TrackingTarget` false))

(event `Tracking`
  (set `self.TrackingTarget` true)
  (`KismetSystemLibrary.Delay` 1.0)
  (`self.Attacking`))

(event `Attacking`
  (`self.Fire Projectile`)
  (`self.Tracking`))

(fn `UserConstructionScript`)