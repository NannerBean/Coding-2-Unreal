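; BP_Melee is an enemy AI Blueprint that tracks health and reacts to damage, working with an AIC_Base controller cached on BeginPlay.
; Taking damage reports an AI damage-sense event at the instigator pawn's location and sends a TookDamage event to the controller's StateTree.
; Damage reduces Health, destroying the actor when depleted, while GETHEALTH adds health clamped to a normalized range.
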(event `self.ReceiveBeginPlay`
  (bind _asaic_base (cast `/Game/Blueprints/EnemyAI/AIC_Base` (`self.GetController`)))
  (set `self.AIC Base` _asaic_base))

(event `self.ReceiveAnyDamage`
  (params (Damage :type "Float (single-precision)") (DamageType :type "DamageType Object Reference") (InstigatedBy :type "Controller Object Reference") (DamageCauser :type "Actor Object Reference"))
  (`AISense_Damage.ReportDamageEvent` self InstigatedBy Damage (`self.K2_GetActorLocation` (`Controller.K2_GetPawn` InstigatedBy)))
  (`StateTreeComponent.SendStateTreeEvent` (`/Game/Blueprints/EnemyAI/AIC_Base.StateTreeAI` (`self.AIC Base`)) (make `StateTreeEvent` (struct :`TagName` "AI.Event.TookDamage")))
  (bind _output_get (set `self.Health` (- (`self.Health`) Damage)))
  (if (not (> _output_get 0.0))
    (`KismetSystemLibrary.PrintText` "I'm so cooked..." true true (struct :`R` 1.0 :`G` 0.275988 :`A` 1.0))
    (`self.K2_DestroyActor`)))

(event `GET HEALTH`
  (params (HealthtoAdd :type "Float (double-precision)"))
  (set `self.Health` (`KismetMathLibrary.FClamp` (+ (`self.Health`) HealthtoAdd))))

(fn `UserConstructionScript`)