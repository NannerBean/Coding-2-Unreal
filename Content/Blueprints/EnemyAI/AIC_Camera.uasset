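; AI controller for security cameras and turrets that relays sight detections to the possessed pawn.
; On possession it caches the pawn as either a BP_SecurityCam or a BP_Turret.
; Perception updates skip actors tagged "AI", print a debug message, and pass sight stimuli to HandleSight.
; HandleSight forwards the sensed state to the cached pawn, adding stimulus location for cameras and the target actor for turrets.
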(event `self.AIPerception.OnTargetPerceptionUpdated`
  (params (Actor :type "Actor Object Reference") (Stimulus :type "AIStimulus Structure"))
  (bind (_age _expirationage _strength _stimuluslocation _receiverlocation _tag _bsuccessfullysensed) (break `AIStimulus` Stimulus))
  (if (not (`self.ActorHasTag` Actor "AI"))
    (bind _returnvalue (`AIPerceptionSystem.GetSenseClassForStimulus` Stimulus))
    (bind _returnvalue_2 (`KismetSystemLibrary.GetClassDisplayName` _returnvalue))
    (`KismetSystemLibrary.PrintText` (`|FormatText` "Sensed {actor} with {name}" Actor _returnvalue_2))
    (switch `name` _tag
      (:`Default`
        (switch `string` _returnvalue_2
          (:`AISense_Sight`
            (`self.HandleSight` Actor _bsuccessfullysensed _stimuluslocation)))))))

(event `self.ReceivePossess`
  (params (PossessedPawn :type "Pawn Object Reference"))
  (bind _asbp_security_cam (cast `/Game/Blueprints/EnemyAI/BP_SecurityCam` PossessedPawn)
    (:`then`
      (set `self.As BP Security Cam` _asbp_security_cam))
    (:`CastFailed`
      (bind _asbp_turret (cast `/Game/Blueprints/EnemyAI/BP_Turret` PossessedPawn))
      (set `self.As BP Turret` _asbp_turret))))

(fn `HandleSight`
  (params (Target :type "Actor Object Reference") (`Successfully Sensed` :type Boolean) (`Stimulus Location` :type "Vector Structure"))
  (bind _as_bp_security_cam (`self.As BP Security Cam`)
    (:`then`
      (`/Game/Blueprints/EnemyAI/BP_SecurityCam.HandleSight` _as_bp_security_cam null `Successfully Sensed` `Stimulus Location`))
    (:`else`
      (bind _as_bp_turret (`self.As BP Turret`)
        (:`then`
          (`/Game/Blueprints/EnemyAI/BP_Turret.Handle Sight` _as_bp_turret Target `Successfully Sensed`))
        (:`else`)))))

(fn `UserConstructionScript`)