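; Battery-powered flashlight item the player can pick up, use and drop with a physics toss.
; Use flip-flops the spotlight while charge remains, starting a self-calling delayed drain that lowers charge until the light cuts out.
; Alternate use spends a battery from the first-person character's counter to restore full charge.
; Automatic shutoff leaves the FlipFlop unreset, so the next Use after recharging takes the off branch.
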(event `self.AlternateUse`
  (bind _returnvalue (`GameplayStatics.GetActorOfClass` "/Game/FirstPerson/Blueprints/BP_FirstPersonCharacter.BP_FirstPersonCharacter_C"))
  (bind _battery_counter (`/Game/FirstPerson/Blueprints/BP_FirstPersonCharacter.Battery Counter` _returnvalue))
  (if (>= _battery_counter 1.0)
    (`KismetSystemLibrary.PrintText` "Used Battery" true true (struct :`R` 1.0 :`G` 0.010377 :`A` 1.0))
    (set `self.Charge` 100.0)
    (set `/Game/FirstPerson/Blueprints/BP_FirstPersonCharacter.Battery Counter` (- _battery_counter 1.0) _returnvalue)
    (set `self.bHasCharge` true)
    (`GameplayStatics.PlaySound2D` "/Game/SFX/764407__tabata_h__changing-batteries-of-a-remote-control.764407__tabata_h__changing-batteries-of-a-remote-control" 1.0 1.0 0.0 null null)
    (else
      (`KismetSystemLibrary.PrintText` "You don't have any batteries..." true true (struct :`R` 1.0 :`G` 0.010377 :`A` 1.0)))))

(event `Drain Battery`
  (`KismetSystemLibrary.Delay` 10.0)
  (if (`self.bIsOn`)
    (bind _output_get (set `self.Charge` (- (`self.Charge`) 10.0)))
    (`KismetSystemLibrary.PrintText` (`|FormatText` "Charge is now at {Charge}" _output_get))
    (if (<= _output_get 0.0)
      (`LightComponent.SetIntensity` (`self.SpotLight`) 0.0)
      (set `self.bIsOn` false)
      (set `self.bHasCharge` false)
      (else
        (`self.Drain Battery`)))))

(event `self.Use`
  (bind _spotlight (`self.SpotLight`))
  (if (`self.bHasCharge`)
    (`/Engine/EditorBlueprintResources/StandardMacros.FlipFlop`
      (:`A`
        (`LightComponent.SetIntensity` _spotlight 8000.0)
        (set `self.bIsOn` true)
        (`GameplayStatics.PlaySound2D` "/Game/SFX/173420__lightyarn__flashlight_on.173420__lightyarn__flashlight_on" 1.0 1.0 0.0 null null)
        (`self.Drain Battery`))
      (:`B`
        (`LightComponent.SetIntensity` _spotlight 0.0)
        (set `self.bIsOn` false)
        (`GameplayStatics.PlaySound2D` "/Game/SFX/173420__lightyarn__flashlight_on.173420__lightyarn__flashlight_on" 1.0 1.0 0.0 null null)))))

(event `self.Pickup`
  (params (Owner :type "/Game/Blueprints/BPC_Interact Object Reference"))
  (`PrimitiveComponent.SetCollisionEnabled` (`self.Box`) "NoCollision"))

(event `self.Drop`
  (bind _box (`self.Box`))
  (`PrimitiveComponent.SetCollisionEnabled` _box "QueryAndPhysics")
  (set `/Game/Blueprints/BPC_Interact.HeldItem` null (stale `self.Pickup` Owner))
  (`PrimitiveComponent.SetSimulatePhysics` _box true)
  (`PrimitiveComponent.AddImpulse` _box (200.0 20.0 50.0) "None" true))

(fn `UserConstructionScript`)