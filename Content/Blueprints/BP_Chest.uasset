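; BP_Chest is an inventory chest that swings its lid open when the first-person character enters its trigger box and shut when they leave.
; A Timeline rotates the hinge, played forward or in reverse by OpenChest.
; Once open, it prints the first item, shows chest and player inventory widgets, and registers BPCInventory with GM_SaveLoad's LevelState.
; LoadInventory sets the component's EnumInventory from a passed-in value.
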(event `self.ReceiveBeginPlay`
  (bind _returnvalue (`|CreateWidget` "/Game/Widgets/WBP_InventoryChestMenu.WBP_InventoryChestMenu_C" null (`self.BPC_Inventory`)))
  (set `self.ChestMenu` _returnvalue))

(event `self.Box.OnComponentBeginOverlap`
  (params (OverlappedComponent :type "PrimitiveComponent Object Reference") (OtherActor :type "Actor Object Reference") (OtherComp :type "PrimitiveComponent Object Reference") (OtherBodyIndex :type Integer) (bFromSweep :type Boolean) (SweepResult :type "HitResult Structure (by ref)"))
  (bind _asbp_first_person_character (cast `/Game/FirstPerson/Blueprints/BP_FirstPersonCharacter` OtherActor))
  (`self.Open Chest` false))

(event `self.Box.OnComponentEndOverlap`
  (params (OverlappedComponent :type "PrimitiveComponent Object Reference") (OtherActor :type "Actor Object Reference") (OtherComp :type "PrimitiveComponent Object Reference") (OtherBodyIndex :type Integer))
  (cast `/Game/FirstPerson/Blueprints/BP_FirstPersonCharacter` OtherActor)
  (`self.Open Chest` true))

(event `Open Chest`
  (params (Reverse :type Boolean))
  (if Reverse
    (bind (_direction _open_chest) (`Timeline|Timeline` :!via `Reverse` :!label _label)
      (:`Update`
        (`SceneComponent.K2_SetRelativeRotation` (`self.RealHinge`) (`KismetMathLibrary.MakeRotator` (`KismetMathLibrary.Lerp` 0.0 -70.0 _open_chest)) false false))
      (:`Finished`
        (if (not Reverse)
          (`KismetSystemLibrary.PrintText` (`|FormatText` "First Item in chest is {name}" (`.Name_2_E47C76FE47613FACC8E998ADAEE5A2E9` (break `/Game/Blueprints/S_Items` (`|GetArrayItem` (`/Game/Blueprints/BPC_Inventory.Inventory` (`self.BPC_Inventory`)))))) true true (struct :`G` 0.66 :`B` 1.0 :`A` 1.0) 10.0)
          (`UserWidget.AddToViewport` (`self.ChestMenu`) 0)
          (`UserWidget.AddToViewport` (`/Game/FirstPerson/Blueprints/BP_FirstPersonCharacter.WBP Player Inventory` (stale `self.Box.OnComponentBeginOverlap` _asbp_first_person_character)) 0)
          (bind _asgm_save_load (cast `/Game/Blueprints/Save_Load/GM_SaveLoad` (`GameplayStatics.GetGameMode`)))
          (`/Game/Blueprints/Save_Load/SG_LevelState.Add Inventory` (`/Game/Blueprints/Save_Load/GM_SaveLoad.LevelState` _asgm_save_load) (`self.BPC_Inventory`)))))
    (else
      (goto _label))))

(event `Load Inventory`
  (params (EnumInventory :type "Array of /Game/Blueprints/E_Items Enum"))
  (set `/Game/Blueprints/BPC_Inventory.EnumInventory` EnumInventory (`self.BPC_Inventory`)))

(fn `UserConstructionScript`)