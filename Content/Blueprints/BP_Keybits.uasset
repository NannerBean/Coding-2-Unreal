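; BP_Keybits is a key-fragment pickup that the first-person character collects on sphere overlap.
; Each pickup increments the character's KeyBitCounter, prints a message and destroys itself.
; At exactly four bits it increments KeyCounter and shows a popup widget, but assigns HasEnoughBitForKey to itself, leaving it unchanged.
; The popup's delayed removal is scheduled after DestroyActor on the same actor, so it likely never runs.
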(event `self.SphereCollision.OnComponentBeginOverlap`
  (params (OverlappedComponent :type "PrimitiveComponent Object Reference") (OtherActor :type "Actor Object Reference") (OtherComp :type "PrimitiveComponent Object Reference") (OtherBodyIndex :type Integer) (bFromSweep :type Boolean) (SweepResult :type "HitResult Structure (by ref)"))
  (bind _asbp_first_person_character (cast `/Game/FirstPerson/Blueprints/BP_FirstPersonCharacter` OtherActor))
  (bind _keybit_counter (`/Game/FirstPerson/Blueprints/BP_FirstPersonCharacter.KeyBit Counter` _asbp_first_person_character))
  (set `/Game/FirstPerson/Blueprints/BP_FirstPersonCharacter.KeyBit Counter` (+ _keybit_counter 1) _asbp_first_person_character)
  (`KismetSystemLibrary.PrintString` "Got Keybit!")
  (`self.K2_DestroyActor`)
  (if (== _keybit_counter 4)
    (set `/Game/FirstPerson/Blueprints/BP_FirstPersonCharacter.bHasEnoughBitForKey` (`/Game/FirstPerson/Blueprints/BP_FirstPersonCharacter.bHasEnoughBitForKey` _asbp_first_person_character) _asbp_first_person_character)
    (`KismetSystemLibrary.PrintString` "You Now have a key!" true true (struct :`R` 1.0 :`G` 0.010059 :`A` 1.0))
    (set `/Game/FirstPerson/Blueprints/BP_FirstPersonCharacter.Key Counter` (+ (`/Game/FirstPerson/Blueprints/BP_FirstPersonCharacter.Key Counter` _asbp_first_person_character) 1) _asbp_first_person_character)
    (bind _returnvalue (`|CreateWidget` "/Game/Widgets/WBP_Popup.WBP_Popup_C"))
    (bind _output_get (set `self.PopUp` _returnvalue))
    (`UserWidget.AddToViewport` _output_get 0)
    (set `EditableTextBox.Text` "The Keybits combined into a key in your hands!" (`/Game/Widgets/WBP_Popup.TextBox` _output_get))
    (`KismetSystemLibrary.Delay` 2.0)
    (`Widget.RemoveFromParent` _output_get)))

(fn `UserConstructionScript`)