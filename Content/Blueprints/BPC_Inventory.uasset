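; BPC_Inventory is an inventory component that stores items as an array of enum values, one per slot.
; GetSlot resolves a slot's enum to its details through GetItemDetailes, which linearly scans DT_Items rows for the matching enum.
; SetSlot writes one slot and fires OnSlotUpdated, while SetEnumInventory replaces the whole array and fires OnRefreshGrid, so listeners can react to either change.
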(fn `GetItemDetailes`
  (params (RequestedItem :type "/Game/Blueprints/E_Items Enum" :default "NewEnumerator0"))
  (returns (ItemDetails :type "/Game/Blueprints/S_Items Structure"))
  (bind _outrownames (`DataTableFunctionLibrary.GetDataTableRowNames` "/Game/Blueprints/DataTables/DT_Items.DT_Items"))
  (for _array_element _outrownames
    (bind _returnvalue (`|GetDataTableRow` "/Game/Blueprints/DataTables/DT_Items.DT_Items" _array_element)
      (:`then`
        (if (`|EnumEquality` (`.Enum_19_DDA48BB54EFAB4B9392D83906DB4EE9E` (break `/Game/Blueprints/S_Items` _returnvalue)) RequestedItem)
          (return _returnvalue))))))

(fn `GetSlot`
  (params (RequestedSlot :type Integer))
  (returns (ItemDetails :type "/Game/Blueprints/S_Items Structure"))
  (bind _itemdetails (`self.GetItemDetailes` (`|GetArrayItem` (`self.EnumInventory`) RequestedSlot)))
  (return _itemdetails))

(fn `SetEnumInventory`
  (params (EnumInventory :type "Array of /Game/Blueprints/E_Items Enum"))
  (set `self.EnumInventory` EnumInventory)
  (`self.OnRefreshGrid`))

(fn `SetSlot`
  (params (Item :type "/Game/Blueprints/E_Items Enum" :default "NewEnumerator3") (`Slot Index` :type Integer))
  (`KismetArrayLibrary.Array_Set` (`self.EnumInventory`) `Slot Index` Item)
  (`self.OnSlotUpdated` `Slot Index`))