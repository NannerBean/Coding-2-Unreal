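; BP_Checkpoint is a checkpoint actor that saves the game when the first-person character overlaps it.
; On BeginPlay it caches the GM_SaveLoad game mode.
; On overlap it passes the character's belt inventory, main inventory, transform and forward vector to that game mode's Save function, then prints a confirmation.
; It has no one-shot guard, so each new overlap saves again.
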(event `self.ReceiveBeginPlay`
  (bind _asgm_save_load (cast `/Game/Blueprints/Save_Load/GM_SaveLoad` (`GameplayStatics.GetGameMode`)))
  (set `self.Game Mode` _asgm_save_load))

(event `self.ReceiveActorBeginOverlap`
  (params (OtherActor :type "Actor Object Reference"))
  (bind _asbp_first_person_character (cast `/Game/FirstPerson/Blueprints/BP_FirstPersonCharacter` OtherActor))
  (`/Game/Blueprints/Save_Load/GM_SaveLoad.Save` (`self.Game Mode`) (`/Game/Blueprints/BPC_Inventory.EnumInventory` (`/Game/FirstPerson/Blueprints/BP_FirstPersonCharacter.BPC_BeltInventory` _asbp_first_person_character)) (`/Game/Blueprints/BPC_Inventory.EnumInventory` (`/Game/FirstPerson/Blueprints/BP_FirstPersonCharacter.BPC_Inventory` _asbp_first_person_character)) (`self.GetTransform` _asbp_first_person_character) (`self.GetActorForwardVector` _asbp_first_person_character))
  (`KismetSystemLibrary.PrintText` "Game Saved"))

(fn `UserConstructionScript`)