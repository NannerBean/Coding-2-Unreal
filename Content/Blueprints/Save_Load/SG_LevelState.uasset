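; SG_LevelState is a level-state object in the save/load system that records activated actors and inventories.
; AddActor and AddInventory add unique entries to their lists.
; Activateactors replays activation by calling ActivateMessage on every recorded actor.
; Inventory restoring is unfinished: LoadInventories is empty, and a map loop over INVActors is left unconnected.
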(event `AddActor`
  (params (Actor :type "Actor Object Reference"))
  (`KismetArrayLibrary.Array_AddUnique` (`self.ActivatedActors`) Actor))

(event `Activate actors`
  (for _array_element (`self.ActivatedActors`)
    (message `/Game/Blueprints/Save_Load/BPI_ActivateActors.Activate` _array_element)))

(event `Add Inventory`
  (params (Inventory :type "/Game/Blueprints/BPC_Inventory Object Reference (by ref)"))
  (`KismetArrayLibrary.Array_AddUnique` (`self.Inventoriess`) Inventory))

(event `Load Inventories`)