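; Game mode that saves and loads player inventory and per-level state through two save objects, SG_Player and SG_LevelState.
; Player data uses the base slot, while level data uses a slot name built with the current level name.
; BeginPlay loads existing saves or creates new objects; Load restores belt, inventory, saved actors, transform and control rotation.
; Delete functions clear slots, then open the level named by SlotName.
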(event `self.ReceiveBeginPlay`
  (`KismetSystemLibrary.PrintText` "Starting GM_SaveLoad" true true (struct :`G` 0.66 :`B` 1.0 :`A` 1.0) 7.0)
  (`|ExecutionSequence`
    (:`then_0`
      (bind _returnvalue (`GameplayStatics.DoesSaveGameExist` (`self.Slot Name`)))
      (if _returnvalue
        (`self.Load`)
        (else
          (bind _returnvalue_2 (`GameplayStatics.CreateSaveGameObject` "/Game/Blueprints/Save_Load/SG_Player.SG_Player_C"))
          (set `self.PlayerSave` _returnvalue_2))))
    (:`then_1`
      (bind _returnvalue_3 (`GameplayStatics.GetCurrentLevelName` true))
      (bind _returnvalue_4 (`GameplayStatics.DoesSaveGameExist` (`KismetStringLibrary.Concat_StrStr` (`self.Slot Name`) "Default_FirstLevel" _returnvalue_3)))
      (if _returnvalue_4
        (`self.Load`)
        (else
          (bind _returnvalue_5 (`GameplayStatics.CreateSaveGameObject` "/Game/Blueprints/Save_Load/SG_LevelState.SG_LevelState_C"))
          (set `self.LevelState` _returnvalue_5))))))

(fn `DeleteLevelSave`
  (bind _slot_name (`self.Slot Name`))
  (bind _returnvalue (`GameplayStatics.GetCurrentLevelName` true))
  (`GameplayStatics.DeleteGameInSlot` (`KismetStringLibrary.Concat_StrStr` _slot_name "Default_FirstLevel" _returnvalue))
  (`GameplayStatics.OpenLevel` (`KismetStringLibrary.Conv_StringToName` _slot_name)))

(fn `DeleteSave`
  (`GameplayStatics.DeleteGameInSlot` (`self.Slot Name`))
  (`self.DeleteLevelSave`))

(fn `Load`
  (bind _playertransform (`/Game/Blueprints/Save_Load/SG_LevelState.PlayerTransform` (`self.LevelState`)))
  (`|ExecutionSequence`
    (:`then_0`
      (bind _returnvalue (`GameplayStatics.LoadGameFromSlot` (`self.Slot Name`)))
      (bind _assg_player (cast `/Game/Blueprints/Save_Load/SG_Player` _returnvalue))
      (set `self.PlayerSave` _assg_player)
      (bind _asbp_first_person_character (cast `/Game/FirstPerson/Blueprints/BP_FirstPersonCharacter` (`GameplayStatics.GetPlayerCharacter` 0)))
      (`/Game/Blueprints/BPC_Inventory.SetEnumInventory` (`/Game/FirstPerson/Blueprints/BP_FirstPersonCharacter.BPC_BeltInventory` _asbp_first_person_character) (`/Game/Blueprints/Save_Load/SG_Player.Belt` (`self.PlayerSave`)))
      (`/Game/Blueprints/BPC_Inventory.SetEnumInventory` (`/Game/FirstPerson/Blueprints/BP_FirstPersonCharacter.BPC_Inventory` _asbp_first_person_character) (`/Game/Blueprints/Save_Load/SG_Player.Player INV` (`self.PlayerSave`)))
      (`KismetSystemLibrary.PrintText` "Inventory Updated"))
    (:`then_1`
      (bind _returnvalue_2 (`GameplayStatics.GetCurrentLevelName` true))
      (bind _returnvalue_3 (`GameplayStatics.LoadGameFromSlot` (`KismetStringLibrary.Concat_StrStr` (`self.Slot Name`) "Default_FirstLevel" _returnvalue_2)))
      (bind _assg_level_state (cast `/Game/Blueprints/Save_Load/SG_LevelState` _returnvalue_3))
      (bind _output_get (set `self.LevelState` _assg_level_state))
      (`/Game/Blueprints/Save_Load/SG_LevelState.Activate actors` _output_get)
      (`/Game/FirstPerson/Blueprints/BP_FirstPersonCharacter.LoadTransform` _asbp_first_person_character _playertransform (0.0 0.0 0.0))
      (`Controller.SetControlRotation` (`GameplayStatics.GetPlayerController` 0) (.rotation _playertransform)))))

(fn `Save`
  (params (Belt :type "Array of /Game/Blueprints/E_Items Enum") (`Player INV` :type "Array of /Game/Blueprints/E_Items Enum") (InputPin :type "Transform Structure") (InputPin1 :type "Vector Structure"))
  (bind _playersave (`self.PlayerSave`))
  ; Save Player Data
  (`|ExecutionSequence`
    (:`then_0`
      (set `/Game/Blueprints/Save_Load/SG_Player.Belt` Belt _playersave)
      (set `/Game/Blueprints/Save_Load/SG_Player.Player INV` `Player INV` _playersave)
      (`GameplayStatics.SaveGameToSlot` (`self.PlayerSave`) (`self.Slot Name`)))
    (:`then_1`
      ; Save Level Data
      (set `/Game/Blueprints/Save_Load/SG_LevelState.PlayerTransform` InputPin (`self.LevelState`))
      (bind _returnvalue (`GameplayStatics.GetCurrentLevelName` true))
      (`GameplayStatics.SaveGameToSlot` (`self.LevelState`) (`KismetStringLibrary.Concat_StrStr` (`self.Slot Name`) "Default_FirstLevel" _returnvalue)))))

(fn `UserConstructionScript`)