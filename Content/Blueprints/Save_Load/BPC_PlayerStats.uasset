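; Player stats component that holds an SPlayerStats struct with health, mana, stamina, gold, experience and a saved location.
; GetCanSprint allows sprinting while stamina is above a small threshold, and Sprinting subtracts a given amount by rebuilding the struct, with no clamping.
; Every tick, DebugStats prints health, mana and stamina on screen for that frame's duration.
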(event `self.ReceiveTick`
  (params (DeltaSeconds :type "Float (single-precision)"))
  (`self.Debug Stats` DeltaSeconds))

(event `Debug Stats`
  (params (Duration :type "Float (double-precision)"))
  (bind (_health _mana _stamina) (break `/Game/Blueprints/Save_Load/S_PlayerStats` (`self.Stats`)))
  (`KismetSystemLibrary.PrintText` (`|FormatText` "HP : {Health}, Mana : {Mana}, Stamina : {Stamina}" _health _mana _stamina) true true (struct :`R` 1.0 :`G` 0.044519 :`A` 1.0) Duration))

(fn `GetCanSprint`
  (returns (`Can Sprint` :type Boolean))
  (bind (_stats_health _stats_mana _stats_stamina) (break `/Game/Blueprints/Save_Load/S_PlayerStats` (`self.Stats`)))
  (return (> _stats_stamina 1.0)))

(fn `Sprinting`
  (params (`ReduceBy:` :type "Float (double-precision)" :default 2.0))
  (bind (_stats_health _stats_mana _stats_stamina _stats_savedlocation _stats_gold _stats_experience) (break `/Game/Blueprints/Save_Load/S_PlayerStats` (`self.Stats`)))
  (set `self.Stats` (make `/Game/Blueprints/Save_Load/S_PlayerStats` _stats_health _stats_mana (- _stats_stamina `ReduceBy:`) _stats_savedlocation _stats_gold _stats_experience)))