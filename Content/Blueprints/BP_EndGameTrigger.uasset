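; BP_EndGameTrigger is a trigger volume that ends the game when the first-person character overlaps it.
; On overlap it calls Stop on the character's FirstPersonMesh, switches the first player controller to UI-only input and shows the mouse cursor.
; It then creates the WBP_END widget, adds it to the viewport and plays its FadeIN animation.
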(event `self.Trigger.OnComponentBeginOverlap`
  (params (OverlappedComponent :type "PrimitiveComponent Object Reference") (OtherActor :type "Actor Object Reference") (OtherComp :type "PrimitiveComponent Object Reference") (OtherBodyIndex :type Integer) (bFromSweep :type Boolean) (SweepResult :type "HitResult Structure (by ref)"))
  (bind _returnvalue (`GameplayStatics.GetPlayerController` 0))
  (bind _asbp_first_person_character (cast `/Game/FirstPerson/Blueprints/BP_FirstPersonCharacter` OtherActor))
  (bind _output_get (set `self.As BP First Person Character` _asbp_first_person_character))
  (`SkeletalMeshComponent.Stop` (`/Game/FirstPerson/Blueprints/BP_FirstPersonCharacter.FirstPersonMesh` _output_get))
  (`WidgetBlueprintLibrary.SetInputMode_UIOnlyEx` _returnvalue null)
  (set `PlayerController.bShowMouseCursor` true _returnvalue)
  (bind _returnvalue_2 (`|CreateWidget` "/Game/Widgets/WBP_END.WBP_END_C"))
  (bind _output_get_2 (set `self.EndScreen` _returnvalue_2))
  (`UserWidget.AddToViewport` _output_get_2 0)
  (`UserWidget.PlayAnimation` _output_get_2 (`/Game/Widgets/WBP_END.FadeIN` _output_get_2) 0.0 1 "Forward" 1.0 false))

(fn `UserConstructionScript`)