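; BP_Camera is an item, apparently a camera prop, that an owner can pick up and drop.
; Pickup stores the owner, disables collision on the Box and returns the item type.
; Drop restores collision, clears the owner's HeldItem, enables physics simulation and throws the Box with a fixed velocity-change impulse that does not depend on the owner's facing.
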(event `/Game/Blueprints/BPI_Item.Drop`
  (bind _box (`self.Box`))
  (`PrimitiveComponent.SetCollisionEnabled` _box "QueryAndPhysics")
  (set `/Game/Blueprints/BPC_Interact.HeldItem` null (`self.Owner_0`))
  (`PrimitiveComponent.SetSimulatePhysics` _box true)
  (`PrimitiveComponent.AddImpulse` _box (200.0 20.0 50.0) "None" true))

(fn `Pickup`
  (params (Owner :type "/Game/Blueprints/BPC_Interact Object Reference"))
  (returns (EItem :type "/Game/Blueprints/E_Items Enum"))
  (set `self.Owner_0` Owner)
  (`PrimitiveComponent.SetCollisionEnabled` (`self.Box`) "NoCollision")
  (return (`self.ItemType`)))

(fn `UserConstructionScript`)