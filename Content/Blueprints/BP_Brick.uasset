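; A held brick item that the player can aim, throw or drop, smashing nearby destructible boxes on impact.
; Alternate use starts a looping timer that draws a predicted projectile arc and arms the throw.
; Use launches the physics box with the same camera-based velocity and updates the belt inventory and hotbar.
; After a throw, non-player hits spawn debris, sphere-trace to destroy BP_DestructibleBox actors with sound, then destroy the brick.
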(event `self.ReceiveBeginPlay`
  (bind _returnvalue (`GameplayStatics.GetActorOfClass` "/Game/FirstPerson/Blueprints/BP_FirstPersonCharacter.BP_FirstPersonCharacter_C"))
  (bind _output_get (set `self.Player` _returnvalue)))

(event `/Game/Blueprints/BPI_Item.Cancel`
  ; Predict Throw Arc
  (`KismetSystemLibrary.K2_ClearAndInvalidateTimerHandle` (stale `/Game/Blueprints/BPI_Item.AlternateUse` _returnvalue))
  (set `self.bCanBeThrown` false))

(event `/Game/Blueprints/BPI_Item.AlternateUse`
  ; Predict Throw Arc
  (bind _returnvalue (`KismetSystemLibrary.K2_SetTimerDelegate` (delegate `Draw Arc`) 0.1 true)))

(event `Draw Arc`
  (bind _returnvalue (`SceneComponent.GetForwardVector` (`/Game/FirstPerson/Blueprints/BP_FirstPersonCharacter.FirstPersonCamera` (`self.Player`))))
  ; Predict Throw Arc
  (bind _predictresult (`GameplayStatics.Blueprint_PredictProjectilePath_Advanced` (make `PredictProjectilePathParams` (`SceneComponent.K2_GetComponentLocation` (`/Game/FirstPerson/Blueprints/BP_FirstPersonCharacter.HandHoldPoint` (`self.Player`))) (`KismetMathLibrary.MakeVector` (.x (* _returnvalue 1000.0)) (.y (* _returnvalue 1000.0)) (* (`KismetMathLibrary.MapRangeUnclamped` (.z _returnvalue) 0.0 1.0 3.0 10.0) 50.0)) true 0.0 1.0 true "ECC_WorldStatic" _ _ 20.0 0.0 "ForDuration" 0.1)))
  (set `self.Predict Result Hit Result` (`.HitResult` (break `PredictProjectilePathResult` _predictresult)))
  (set `self.bCanBeThrown` true))

(event `/Game/Blueprints/BPI_Item.Use`
  (bind _box (`self.Box`))
  (bind _player (`self.Player`))
  (bind _returnvalue (`SceneComponent.GetForwardVector` (`/Game/FirstPerson/Blueprints/BP_FirstPersonCharacter.FirstPersonCamera` (`self.Player`))))
  ; Throw
  (if (`self.bCanBeThrown`)
    (`PrimitiveComponent.SetCollisionEnabled` _box "QueryAndPhysics")
    (set `/Game/Blueprints/BPC_Interact.HeldItem` null (`self.Owner_0`))
    (`PrimitiveComponent.SetSimulatePhysics` _box true)
    (`PrimitiveComponent.AddImpulse` _box (`KismetMathLibrary.MakeVector` (.x (* _returnvalue 1000.0)) (.y (* _returnvalue 1000.0)) (* (`KismetMathLibrary.MapRangeUnclamped` (.z _returnvalue) 0.0 1.0 3.0 10.0) 50.0)) "None" true)
    (`/Game/Blueprints/BPC_Inventory.SetSlot` (`/Game/FirstPerson/Blueprints/BP_FirstPersonCharacter.BPC_BeltInventory` _player) "NewEnumerator3" (`/Game/Blueprints/BPC_Interact.Active Slot` (`/Game/FirstPerson/Blueprints/BP_FirstPersonCharacter.BPC_Interact` _player)))
    (`/Game/Widgets/WBP_InventoryGrid.Refresh Grid` (`/Game/Widgets/WBP_BELT.WBP_Hotbar` (`/Game/FirstPerson/Blueprints/BP_FirstPersonCharacter.WBPBeltWidget` _player)))
    (set `self.bWas Thrown` true)
    (set `self.bCanBeThrown` false)
    (set `/Game/FirstPerson/Blueprints/BP_FirstPersonCharacter.bHasHeldItem` false (`self.Player`))
    (`/Game/Blueprints/BPI_Item.Cancel`)))

(event `/Game/Blueprints/BPI_Item.Drop`
  (bind _box (`self.Box`))
  (`PrimitiveComponent.SetCollisionEnabled` _box "QueryAndPhysics")
  (set `/Game/Blueprints/BPC_Interact.HeldItem` null (`self.Owner_0`))
  (`PrimitiveComponent.SetSimulatePhysics` _box true)
  (`PrimitiveComponent.AddImpulse` _box (200.0 20.0 50.0) "None" true))

(event `self.Box.OnComponentHit`
  (params (HitComponent :type "PrimitiveComponent Object Reference") (OtherActor :type "Actor Object Reference") (OtherComp :type "PrimitiveComponent Object Reference") (NormalImpulse :type "Vector Structure") (Hit :type "HitResult Structure (by ref)"))
  (bind (_bblockinghit _binitialoverlap _time _distance _location _impactpoint) (`GameplayStatics.BreakHitResult` Hit))
  ; At impact point, spawn particles and break destrctibles
  (cast `/Game/FirstPerson/Blueprints/BP_FirstPersonCharacter` OtherActor
    (:`CastFailed`
      (if (`self.bWas Thrown`)
        (`KismetSystemLibrary.PrintText` "Brick hit something" true true (struct :`R` 1.0 :`B` 0.009271 :`A` 1.0))
        (`NiagaraFunctionLibrary.SpawnSystemAtLocation` "/Game/VFX/NS_BrickDebris.NS_BrickDebris" _impactpoint)
        (bind _outhits (`KismetSystemLibrary.SphereTraceMulti` :`Start` _impactpoint :`Radius` 100.0 :`TraceChannel` "TraceTypeQuery1" :`DrawDebugType` "ForDuration"))
        (for _array_element _outhits
          (bind _asbp_destructible_box (cast `/Game/Blueprints/BP_DestructibleBox` (`.HitActor` (`GameplayStatics.BreakHitResult` _array_element))))
          (`self.K2_DestroyActor` _asbp_destructible_box)
          (`GameplayStatics.PlaySoundAtLocation` "/Game/SFX/437602__debsound__brick-debris-fall-06.437602__debsound__brick-debris-fall-06" _impactpoint (struct) 1.0 1.0 0.0 null null null null))
        (`self.K2_DestroyActor`)))))

(fn `Pickup`
  (params (Owner :type "/Game/Blueprints/BPC_Interact Object Reference"))
  (returns (EItem :type "/Game/Blueprints/E_Items Enum"))
  (set `self.Owner_0` Owner)
  (`PrimitiveComponent.SetCollisionEnabled` (`self.Box`) "NoCollision")
  (return (`self.ItemType`)))

(fn `UserConstructionScript`)