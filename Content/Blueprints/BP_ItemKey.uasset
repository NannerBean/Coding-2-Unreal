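; BP_ItemKey is a key item the player can pick up, drop, or use to open a door.
; Pickup stores the owner, disables Box collision, registers the actor with GM_SaveLoad's LevelState and returns its item type.
; Use traces forward from the Box; hitting a BP_InteractDoor opens it, clears the held item and destroys the key.
; Drop restores collision and physics with an impulse, while Activate destroys the actor after a zero delay.
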(event `/Game/Blueprints/BPI_Item.Use`
  (bind _box (`self.Box`))
  (bind _returnvalue (`SceneComponent.K2_GetComponentLocation` _box))
  (bind _outhit (`KismetSystemLibrary.LineTraceSingle` :`Start` _returnvalue :`End` (+ _returnvalue (* (`SceneComponent.GetForwardVector` _box) 300.0)) :`TraceChannel` "TraceTypeQuery1" :`DrawDebugType` "ForDuration"))
  (bind _asbp_interact_door (cast `/Game/Blueprints/BP_InteractDoor` (`.HitActor` (`GameplayStatics.BreakHitResult` _outhit))))
  (set `/Game/Blueprints/BPC_Interact.HeldItem` null (`self.Owner_0`))
  (bind _returnvalue_2 (`GameplayStatics.GetActorOfClass` "/Game/FirstPerson/Blueprints/BP_FirstPersonCharacter.BP_FirstPersonCharacter_C"))
  (set `/Game/FirstPerson/Blueprints/BP_FirstPersonCharacter.bHasHeldItem` false _returnvalue_2)
  (`/Game/Blueprints/BP_InteractDoor.Open Door` _asbp_interact_door)
  (`self.K2_DestroyActor`))

(event `/Game/Blueprints/BPI_Item.Drop`
  (bind _box (`self.Box`))
  (`PrimitiveComponent.SetCollisionEnabled` _box "QueryAndPhysics")
  (set `/Game/Blueprints/BPC_Interact.HeldItem` null (`self.Owner_0`))
  (`PrimitiveComponent.SetSimulatePhysics` _box true)
  (`PrimitiveComponent.AddImpulse` _box (200.0 20.0 50.0) "None" true))

(event `/Game/Blueprints/Save_Load/BPI_ActivateActors.Activate`
  (`KismetSystemLibrary.Delay` 0.0)
  (`self.K2_DestroyActor`))

(fn `Pickup`
  (params (Owner :type "/Game/Blueprints/BPC_Interact Object Reference"))
  (returns (EItem :type "/Game/Blueprints/E_Items Enum"))
  (set `self.Owner_0` Owner)
  (`PrimitiveComponent.SetCollisionEnabled` (`self.Box`) "NoCollision")
  (bind _asgm_save_load (cast `/Game/Blueprints/Save_Load/GM_SaveLoad` (`GameplayStatics.GetGameMode`)))
  (`/Game/Blueprints/Save_Load/SG_LevelState.AddActor` (`/Game/Blueprints/Save_Load/GM_SaveLoad.LevelState` _asgm_save_load) self)
  (return (`self.ItemType`)))

(fn `UserConstructionScript`)