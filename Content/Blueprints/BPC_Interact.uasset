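; Player interaction component for BP_FirstPersonCharacter that handles picking up, using, dropping and hotbar-swapping held items.
; A self-repeating, delayed sphere trace from the camera tracks the last BPI_Item actor in view.
; Key and mouse input attach that item to the hand or send it use, cancel and drop messages, syncing pickups and drops to the belt inventory.
; Hotbar swaps destroy the held actor and spawn the new slot's class.
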(event `self.ReceiveBeginPlay`
  (bind _asbp_first_person_character (cast `/Game/FirstPerson/Blueprints/BP_FirstPersonCharacter` (`self.GetOwner`)))
  (set `self.Player` _asbp_first_person_character)
  (set `self.First Person Camera` (`/Game/FirstPerson/Blueprints/BP_FirstPersonCharacter.FirstPersonCamera` _asbp_first_person_character))
  (`self.Looking`)
  (`self.Swap Active item` 0))

(event `Looking`
  (bind _first_person_camera (`self.First Person Camera`))
  (bind _returnvalue (`SceneComponent.K2_GetComponentLocation` _first_person_camera))
  ; Looking for objects to interact with
  (`KismetSystemLibrary.Delay` (`self.LookInterval`))
  (bind (_outhit _returnvalue_2) (`KismetSystemLibrary.SphereTraceSingle` :`Start` _returnvalue :`End` (+ _returnvalue (* (`SceneComponent.GetForwardVector` _first_person_camera) 300.0)) :`Radius` 50.0 :`TraceChannel` "TraceTypeQuery1" :`TraceColor` (struct :`R` 1.0 :`B` 0.105334 :`A` 1.0) :`TraceHitColor` (struct :`R` 0.427976 :`G` 1.0 :`B` 0.200411 :`A` 1.0) :`DrawTime` 1.0))
  (if _returnvalue_2
    (bind (_bblockinghit _binitialoverlap _time _distance _location _impactpoint _normal _impactnormal _physmat _hitactor) (`GameplayStatics.BreakHitResult` _outhit))
    (if (`KismetSystemLibrary.DoesImplementInterface` _hitactor "/Game/Blueprints/BPI_Item.BPI_Item_C")
      (set `self.Last Touched Item` _hitactor)
      (`KismetSystemLibrary.PrintText` (`|FormatText` "Press E to Pickup {name} !" (`KismetSystemLibrary.GetDisplayName` _hitactor)) true true (struct :`G` 0.66 :`B` 1.0 :`A` 1.0) 0.1)
      (else
        (set `self.Last Touched Item` null)))
    (else
      (set `self.Last Touched Item` null)))
  (`self.Looking`))

(event `Key|E`
  (params (Key :type "Key Structure"))
  ; Pickup Item and attach to hand mesh
  (:`Pressed`
    (if (`/Game/FirstPerson/Blueprints/BP_FirstPersonCharacter.bHasHeldItem` (`self.Player`))
      (`KismetSystemLibrary.PrintText` "You're already holding something...")
      (else
        (`self.Try to pick up`)))))

(event `Try to pick up`
  (bind _player (`self.Player`))
  ; Pickup Item and attach to hand mesh
  (bind _last_touched_item (`self.Last Touched Item`)
    (:`then`
      (bind _eitem (message `/Game/Blueprints/BPI_Item.Pickup` _last_touched_item self))
      (`Actor.K2_AttachToComponent` _last_touched_item (`/Game/FirstPerson/Blueprints/BP_FirstPersonCharacter.HandHoldPoint` (`self.Player`)) "None" "SnapToTarget" "SnapToTarget" "KeepRelative" true)
      (set `self.HeldItem` _last_touched_item)
      (set `/Game/FirstPerson/Blueprints/BP_FirstPersonCharacter.bHasHeldItem` true (`self.Player`))
      (`/Game/Blueprints/BPC_Inventory.SetSlot` (`/Game/FirstPerson/Blueprints/BP_FirstPersonCharacter.BPC_BeltInventory` _player) _eitem (`self.Active Slot`))
      (`/Game/Widgets/WBP_InventoryGrid.Refresh Grid` (`/Game/Widgets/WBP_BELT.WBP_Hotbar` (`/Game/FirstPerson/Blueprints/BP_FirstPersonCharacter.WBPBeltWidget` _player))))
    (:`else`
      (`KismetSystemLibrary.PrintText` "We're not looking at anything"))))

(event `Key|LeftMouseButton`
  (params (Key :type "Key Structure"))
  ; Try to use held Item
  (:`Pressed`
    (`self.Try to Use`)))

(event `Key|RightMouseButton`
  (params (Key :type "Key Structure"))
  ; Try to use held item (Alternate use)
  (:`Pressed`
    (`self.Try to use (Alternate)`))
  (:`Released`
    (`self.Cancel Use`)))

(event `Try to Use`
  ; Try to use held Item
  (bind _helditem (`self.HeldItem`)
    (:`then`
      (message `/Game/Blueprints/BPI_Item.Use` _helditem))
    (:`else`
      (`KismetSystemLibrary.PrintText` "You aren't holding anything."))))

(event `Try to use (Alternate)`
  ; Try to use held item (Alternate use)
  (bind _helditem (`self.HeldItem`)
    (:`then`
      (message `/Game/Blueprints/BPI_Item.AlternateUse` _helditem))
    (:`else`
      (`KismetSystemLibrary.PrintText` "Alt use... what?"))))

(event `Cancel Use`
  (bind _helditem (`self.HeldItem`)
    (:`then`
      (message `/Game/Blueprints/BPI_Item.Cancel` _helditem))
    (:`else`)))

(event `Key|Q`
  (params (Key :type "Key Structure"))
  ; Drop held Item
  (:`Pressed`
    (`self.Try to Drop`)))

(event `Try to Drop`
  (bind _player (`self.Player`))
  ; Drop held Item
  (bind _helditem (`self.HeldItem`)
    (:`then`
      (message `/Game/Blueprints/BPI_Item.Drop` _helditem)
      (`/Game/Blueprints/BPC_Inventory.SetSlot` (`/Game/FirstPerson/Blueprints/BP_FirstPersonCharacter.BPC_BeltInventory` _player) "NewEnumerator3" (`self.Active Slot`))
      (`/Game/Widgets/WBP_InventoryGrid.Refresh Grid` (`/Game/Widgets/WBP_BELT.WBP_Hotbar` (`/Game/FirstPerson/Blueprints/BP_FirstPersonCharacter.WBPBeltWidget` _player)))
      (set `/Game/FirstPerson/Blueprints/BP_FirstPersonCharacter.bHasHeldItem` false (`self.Player`)))
    (:`else`)))

(event `Swap Active item`
  (params (NewSlotIndex :type Integer))
  (bind _handholdpoint (`/Game/FirstPerson/Blueprints/BP_FirstPersonCharacter.HandHoldPoint` (`self.Player`)))
  ; Spawn From Hotbar
  (if (!= NewSlotIndex (`self.Active Slot`))
    (bind _output_get (set `self.Active Slot` NewSlotIndex))
    (bind _helditem (`self.HeldItem`)
      (:`then`
        (`Actor.K2_DestroyActor` _helditem))
      (:`else`
        _))
    (bind (_enum _name _description _uiimage _actorbp) (break `/Game/Blueprints/S_Items` (`/Game/Blueprints/BPC_Inventory.GetSlot` (`/Game/FirstPerson/Blueprints/BP_FirstPersonCharacter.BPC_BeltInventory` (`self.Player`)) _output_get)))
    (if (`|EnumInequality` _enum "NewEnumerator3")
      (bind _returnvalue (`|SpawnActorFromClass` _actorbp (`SceneComponent.GetRelativeTransform` _handholdpoint) "Undefined" "MultiplyWithRoot" null null))
      (bind _output_get_2 (set `self.HeldItem` _returnvalue))
      (message `/Game/Blueprints/BPI_Item.Pickup` _output_get_2 self)
      (`Actor.K2_AttachToComponent` _output_get_2 _handholdpoint "None" "SnapToTarget" "SnapToTarget" "KeepRelative" true)
      (else
        (set `self.HeldItem` null)
        (`Actor.K2_DestroyActor` (`self.HeldItem`))))))

(event `Key|One`
  (params (Key :type "Key Structure"))
  ; Spawn From Hotbar
  (:`Pressed`
    (`self.Swap Active item` 0)))

(event `Key|Two`
  (params (Key :type "Key Structure"))
  ; Spawn From Hotbar
  (:`Pressed`
    (`self.Swap Active item` 1)))

(event `Key|Three`
  (params (Key :type "Key Structure"))
  ; Spawn From Hotbar
  (:`Pressed`
    (`self.Swap Active item` 2)))